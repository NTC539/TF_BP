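; Gameplay Ability that lets a crouched character slide while moving fast.
; On activation it requires a minimum horizontal speed, then zeroes the movement component's friction and braking deceleration.
; A looping timer set to the current frame delta acts as a tick, ending the ability when speed drops or crouch is released.
; Ending restores hard-coded friction and braking values, not cached ones, and sets Walking mode.
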(event Custom|Tick
  (bind _returnvalue (Ability|GetOwningActorfromActorInfo))
  (bind _returnvalue_2 (Transformation|GetVelocity _returnvalue))
  (if (not (and (>= (Math|Vector|VectorLength (Math|Vector|MakeVector (.x _returnvalue_2) (.y _returnvalue_2) 0.0)) 4e+02) (Variables|/Script/Engine.Character|GetbIsCrouched (stale Ability|EventActivateAbility _ascharacter))))
    (Ability|EndAbility)))

(event Ability|EventActivateAbility
  (bind _returnvalue (Ability|GetOwningActorfromActorInfo))
  (bind _returnvalue_2 (Transformation|GetVelocity _returnvalue))
  (bind _returnvalue_3 (Actor|GetComponentbyClass _returnvalue "/Script/Engine.CharacterMovementComponent"))
  (bind _ascharacter (Utilities|Casting|CastToCharacter _returnvalue))
  (if (>= (Math|Vector|VectorLength (Math|Vector|MakeVector (.x _returnvalue_2) (.y _returnvalue_2) 0.0)) 4e+02)
    (Utilities|IsValid _returnvalue_3
      (:Is%20Valid
        (Variables|/Script/Engine.CharacterMovementComponent|SetBrakingFriction _returnvalue_3 0.0)
        (Variables|/Script/Engine.CharacterMovementComponent|SetGroundFriction _returnvalue_3 0.0)
        (Variables|/Script/Engine.CharacterMovementComponent|SetBrakingDecelerationWalking _returnvalue_3 0.0)
        (Variables|/Script/Engine.CharacterMovementComponent|SetBrakingDecelerationFalling _returnvalue_3 0.0)
        (bind _returnvalue_4 (Utilities|Time|SetTimerbyEvent (delegate Custom|Tick) (Utilities|Time|GetWorldDeltaSeconds) true))
        (Variables|Default|SetTickTimer _returnvalue_4)))
    (else
      (Ability|EndAbility))))

(event Ability|EventOnEndAbility
  (params (bWasCancelled :type Boolean))
  (bind _returnvalue (Ability|GetOwningActorfromActorInfo))
  (bind _returnvalue_2 (Actor|GetComponentbyClass _returnvalue "/Script/Engine.CharacterMovementComponent"))
  (Utilities|IsValid _returnvalue_2
    (:Is%20Valid
      (Variables|/Script/Engine.CharacterMovementComponent|SetBrakingFriction _returnvalue_2 2.0)
      (Variables|/Script/Engine.CharacterMovementComponent|SetGroundFriction _returnvalue_2 8.0)
      (Variables|/Script/Engine.CharacterMovementComponent|SetBrakingDecelerationWalking _returnvalue_2 2048.0)
      (Variables|/Script/Engine.CharacterMovementComponent|SetBrakingDecelerationFalling _returnvalue_2 2048.0)
      (Pawn|Components|CharacterMovement|SetMovementMode _returnvalue_2 "MOVE_Walking" 0))))